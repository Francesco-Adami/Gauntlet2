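; BP_Bullet is a pooled projectile actor, switched on and off through Activate and Deactivate events instead of being spawned and destroyed.
; Activate teleports it to the supplied pool transform, enables tick, visibility and collision, then passes the projectile direction to SetDirection, which is defined outside these graphs.
; Deactivate teleports it to the return transform and disables all three.
; Activate also prints the direction as debug output.
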(event `ObjectPoolInterface.BP_Activate`
  (params (Data :type "ObjectPoolActivateData Structure"))
  (bind (_objectpooltransform _projectiledir) (break `ObjectPoolActivateData` Data))
  (`KismetSystemLibrary.PrintString` (`KismetStringLibrary.Conv_VectorToString` _projectiledir))
  (`self.K2_SetActorTransform` _objectpooltransform false true)
  (`self.SetActorTickEnabled` true)
  (`self.SetActorHiddenInGame` false)
  (`self.SetActorEnableCollision` true)
  (`self.SetDirection` _projectiledir))

(event `ObjectPoolInterface.BP_Deactivate`
  (params (Data :type "ObjectPoolDeactivateData Structure"))
  (`self.K2_SetActorTransform` (`.ObjectPoolReturnTransform` (break `ObjectPoolDeactivateData` Data)) false true)
  (`self.SetActorTickEnabled` false)
  (`self.SetActorHiddenInGame` true)
  (`self.SetActorEnableCollision` false))

(fn `UserConstructionScript`)